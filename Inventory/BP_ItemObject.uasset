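; BP_ItemObject is an inventory item object that exposes the data describing one item.
; It holds that data in a single Parameters struct, with getters for the item's dimensions, icon and class, plus one returning the whole struct.
; The graphs contain only these accessors, with no logic that sets or changes the data.
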(fn GetDimensions
  (return (.dimensions (Variables|Default|GetParameters))))

(fn GetIcon
  (return (.icon (Variables|Default|GetParameters))))

(fn GetItemClass
  (return (.class_ob (Variables|Default|GetParameters))))

(fn GetParameters
  (return (Variables|Default|GetParameters)))