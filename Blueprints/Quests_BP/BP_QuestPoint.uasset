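; BP_QuestPoint is a placeable trigger that gives or completes a quest when the MyMainCharacter walks into its box.
; On overlap while Activate is set, the Completed flag picks whether the player character completes or adds the Quest, showing its widget.
; It then clears Activate so it fires once, and exposes SaveName through GetUniqueSaveName.
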(event OnComponentBeginOverlap(Box)
  (params (OverlappedComponent :type Primitive%20Component%20Object%20Reference) (OtherActor :type Actor%20Object%20Reference) (OtherComp :type Primitive%20Component%20Object%20Reference) (OtherBodyIndex :type Integer) (bFromSweep :type Boolean) (SweepResult :type Hit%20Result%20Structure%20%28by%20ref%29))
  (bind _quest (Variables|Default|GetQuest))
  (Utilities|Casting|CastToMyMainCharacter OtherActor)
  (if (Variables|Default|GetActivate)
    (if (Variables|Default|GetCompleted?)
      (bind _asmy_main_character (Utilities|Casting|CastToMyMainCharacter (Game|GetPlayerCharacter 0)))
      (Default|CompletedQuestandShowWidget _asmy_main_character _quest)
      (Variables|Default|SetActivate false)
      (else
        (bind _asmy_main_character_2 (Utilities|Casting|CastToMyMainCharacter (Game|GetPlayerCharacter 0)))
        (Default|AddQuestandShowWidget _asmy_main_character_2 _quest)
        (Variables|Default|SetActivate false)))))

(fn ConstructionScript)

(fn GetUniqueSaveName
  (return (Variables|Default|GetSaveName)))