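; BP_Lamp_One is a lamp Blueprint whose SpotLight starts shown or hidden to match the state of a referenced Switcher.
; On BeginPlay it calls the parent, then, if Switcher is valid, copies its On flag to the light's visibility without propagating to children.
; The state is read only once here; Tick and overlap events are disabled stubs, and the construction script only calls its parent.
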(event EventBeginPlay
  (|CallParentFunction)
  (bind _switcher (Variables|Default|GetSwitcher)
    (:then
      (if (Variables|/Game/ThirdPerson/Blueprints/Active_Meshes/Mesh_Active_Switcher.Mesh_Active_Switcher_C|GetOn? _switcher)
        (Rendering|SetVisibility (Variables|Default|GetSpotLight) true false)
        (else
          (Rendering|SetVisibility (Variables|Default|GetSpotLight) false false))))
    (:else)))

(event Collision|EventActorBeginOverlap
  (params (OtherActor :type Actor%20Object%20Reference))
  (|CallParentFunction OtherActor) ; This node is disabled and will not be called.\nDrag off pins to build functionality.
)

(event EventTick
  (params (DeltaSeconds :type Float%20%28single-precision%29))
  (|CallParentFunction DeltaSeconds) ; This node is disabled and will not be called.\nDrag off pins to build functionality.
)

(fn ConstructionScript
  (|CallParentFunction))