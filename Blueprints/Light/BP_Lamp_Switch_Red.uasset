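; BP_Lamp_Switch_Red is a lamp hazard that lights up near the player and kills a player who lacks the required item.
; ActivateTrigger shows the SpotLight while a MyMainCharacter overlaps it and hides it on exit.
; On overlap, DeadTrigger scans the character's InventoryComponent for a specific item ID and calls Kill if none matches.
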(event OnActorBeginOverlap(ActivateTrigger)
  (params (OverlappedActor :type Actor%20Object%20Reference) (OtherActor :type Actor%20Object%20Reference))
  (Utilities|Casting|CastToMyMainCharacter OtherActor)
  (Rendering|SetVisibility (Variables|Default|GetSpotLight) true false))

(event OnActorEndOverlap(ActivateTrigger)
  (params (OverlappedActor :type Actor%20Object%20Reference) (OtherActor :type Actor%20Object%20Reference))
  (Utilities|Casting|CastToMyMainCharacter OtherActor)
  (Rendering|SetVisibility (Variables|Default|GetSpotLight) false false))

(event OnActorBeginOverlap(DeadTrigger)
  (params (OverlappedActor :type Actor%20Object%20Reference) (OtherActor :type Actor%20Object%20Reference))
  (bind _asmy_main_character (Utilities|Casting|CastToMyMainCharacter OtherActor))
  (bind _array_element (Utilities|Array|ForEachLoopwithBreak (Variables|/Game/Inventory/Inventory_Component.Inventory_Component_C|GetItems (Variables|/Game/ThirdPerson/Blueprints/MyMainCharacter.MyMainCharacter_C|GetInventoryComponent _asmy_main_character)) :!label _label)
    (:LoopBody
      (if (== (.id_item (Variables|/Game/Inventory/BP_ItemObject.BP_ItemObject_C|GetParameters _array_element)) 3)
        (Variables|Default|SetFind true)
        (goto _label Break)))
    (:Completed
      (if (Variables|Default|GetFind)
        _
        (else
          (Default|Kill _asmy_main_character)))
      (Variables|Default|SetFind false))))

(event EventBeginPlay
  (|CallParentFunction)
  (bind _asmy_main_character (Utilities|Casting|CastToMyMainCharacter (Game|GetPlayerCharacter 0)))
  (Variables|Default|SetAs%20My%20Main%20Character _asmy_main_character))

(event Collision|EventActorBeginOverlap
  (params (OtherActor :type Actor%20Object%20Reference))
  (|CallParentFunction OtherActor) ; This node is disabled and will not be called.\nDrag off pins to build functionality.
)

(event EventTick
  (params (DeltaSeconds :type Float%20%28single-precision%29))
  (|CallParentFunction DeltaSeconds) ; This node is disabled and will not be called.\nDrag off pins to build functionality.
)

(fn ConstructionScript
  (|CallParentFunction))